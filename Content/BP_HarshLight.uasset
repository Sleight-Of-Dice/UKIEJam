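; Harsh light beam hazard that periodically switches on and off, damaging the 2D side-scroller player inside it.
; A looping timer, its interval randomized in the construction script, flip-flops a timeline that fades both cylinders' shared dynamic material and toggles On.
; While on, Tick calls Damage with random ambient sounds for overlaps on Cylinder, and GROWHARSH for overlaps on Cylinder1.
; Both overlap flags only set if the beam is on at entry.
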(event OnComponentBeginOverlap(Cylinder1)
  (params (OverlappedComponent :type Primitive%20Component%20Object%20Reference) (OtherActor :type Actor%20Object%20Reference) (OtherComp :type Primitive%20Component%20Object%20Reference) (OtherBodyIndex :type Integer) (bFromSweep :type Boolean) (SweepResult :type Hit%20Result%20Structure%20%28by%20ref%29))
  ;[1 1 1] Overlapping Harsh
  (if (Variables|Default|GetOn)
    (Utilities|Casting|CastTo2DSideScrollerCharacter OtherActor
      (:then
        (Variables|Default|SetOverlappingHarsh true))
      (:CastFailed
        (Variables|Default|SetOverlappingHarsh false :!label _label)))
    (else
      (goto _label))))

(event OnComponentEndOverlap(Cylinder1)
  (params (OverlappedComponent :type Primitive%20Component%20Object%20Reference) (OtherActor :type Actor%20Object%20Reference) (OtherComp :type Primitive%20Component%20Object%20Reference) (OtherBodyIndex :type Integer))
  ;[1 1 1] Overlapping Harsh
  (Utilities|Casting|CastTo2DSideScrollerCharacter OtherActor
    (:then
      _)
    (:CastFailed
      _))
  (Variables|Default|SetOverlappingHarsh false))

(event OnComponentBeginOverlap(Cylinder)
  (params (OverlappedComponent :type Primitive%20Component%20Object%20Reference) (OtherActor :type Actor%20Object%20Reference) (OtherComp :type Primitive%20Component%20Object%20Reference) (OtherBodyIndex :type Integer) (bFromSweep :type Boolean) (SweepResult :type Hit%20Result%20Structure%20%28by%20ref%29))
  ;[1 1 1] Damage Overlap
  (if (Variables|Default|GetOn)
    (Utilities|Casting|CastTo2DSideScrollerCharacter OtherActor
      (:then
        (Variables|Default|SetOverlappingDamage true))
      (:CastFailed
        (Variables|Default|SetOverlappingDamage false :!label _label)
        (Variables|Default|SetPlay%20Sound true)))
    (else
      (goto _label))))

(event OnComponentEndOverlap(Cylinder)
  (params (OverlappedComponent :type Primitive%20Component%20Object%20Reference) (OtherActor :type Actor%20Object%20Reference) (OtherComp :type Primitive%20Component%20Object%20Reference) (OtherBodyIndex :type Integer))
  ;[1 1 1] Damage Overlap
  (Utilities|Casting|CastTo2DSideScrollerCharacter OtherActor
    (:then
      _)
    (:CastFailed
      _))
  (Variables|Default|SetOverlappingDamage false)
  (Variables|Default|SetPlay%20Sound true))

(event Custom|FadeInOrOut
  (bind _fadeinandout (Variables|Default|GetFadeInAndOut))
  (Utilities|FlowControl|FlipFlop
    (:A
      (Audio|Components|Audio|Play _fadeinandout)
      (Variables|Default|SetOn true))
    (:B
      (Utilities|String|Reverse _fadeinandout)
      (Variables|Default|SetOn false))))

(event EventBeginPlay
  (bind _returnvalue (Rendering|Material|CreateDynamicMaterialInstance "/Game/MI_LightBeam.MI_LightBeam" "None" :!class /Script/Engine.KismetMaterialLibrary))
  (Variables|Default|SetDynamicMaterial _returnvalue)
  (Rendering|Material|SetMaterial (Variables|Default|GetCylinder) 0 (Variables|Default|GetDynamicMaterial))
  (Rendering|Material|SetMaterial (Variables|Default|GetCylinder1) 0 (Variables|Default|GetDynamicMaterial))
  (Utilities|Time|SetTimerbyEvent (delegate Custom|FadeInOrOut) (Variables|Default|GetFade) true))

(event EventTick
  (params (DeltaSeconds :type Float%20%28single-precision%29))
  (bind _returnvalue (Game|Player|GetPlayerPawn 0))
  (bind _as2dside_scroller_character (Utilities|Casting|CastTo2DSideScrollerCharacter _returnvalue))
  (if (Variables|Default|GetOn)
    (Variables|Default|SetbGenerateOverlapEventsDuringLevelStreaming true)
    (if (Variables|Default|GetOverlappingDamage)
      (Utilities|FlowControl|Sequence
        (:then_0
          (if true
            (Variables|Default|SetPlay%20Sound false)
            (switch int (Math|Random|RandomInteger 3)
              (:0
                (Audio|PlaySoundatLocation "/Game/2DSideScroller/Assets/Sounds/Light_Ambient_1.Light_Ambient_1" "0, 0, 0" "0, 0, 0" 1.0 1.0 0.0 0 0 0))
              (:1
                (Audio|PlaySoundatLocation "/Game/2DSideScroller/Assets/Sounds/Light_Ambient_2.Light_Ambient_2" "0, 0, 0" "0, 0, 0" 1.0 1.0 0.0 0 0 0))
              (:2
                (Audio|PlaySoundatLocation "/Game/2DSideScroller/Assets/Sounds/Light_Ambient_3.Light_Ambient_3" "0, 0, 0" "0, 0, 0" 1.0 1.0 0.0 0 0 0)))
            (Utilities|FlowControl|Delay 0.2)
            (Variables|Default|SetPlay%20Sound true)))
        (:then_1
          (Default|Damage _as2dside_scroller_character)
          (if (Variables|Default|GetOverlappingHarsh) :!label _label
            (Default|GROWHARSH _as2dside_scroller_character))))
      (else
        (goto _label)))
    (else
      (Variables|Default|SetbGenerateOverlapEventsDuringLevelStreaming false))))

(fn ConstructionScript
  (Variables|Default|SetFade (Math|Conversions|ToFloat(Integer) (Math|Integer|Clamp(Integer) (Math|Random|RandomInteger 37) 5 10))))