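; BP_SoftLight is a wandering actor for a 2D side-scroller that triggers GrowSoft on the player while overlapped.
; Every tick it offsets along world X, with a Direction flag setting the sign of its speed.
; A tick counter periodically re-rolls speed and direction, skipping movement and growth on that tick.
; Character overlap events toggle a flag that Tick checks before calling GrowSoft on player pawn 0.
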(event Collision|EventActorBeginOverlap
  (params (OtherActor :type Actor%20Object%20Reference))
  (Utilities|Casting|CastTo2DSideScrollerCharacter OtherActor)
  (Variables|Default|SetOverlappingSoft true))

(event Collision|EventActorEndOverlap
  (params (OtherActor :type Actor%20Object%20Reference))
  (Utilities|Casting|CastTo2DSideScrollerCharacter OtherActor)
  (Variables|Default|SetOverlappingSoft false))

(event EventTick
  (params (DeltaSeconds :type Float%20%28single-precision%29))
  (if (Variables|Default|GetDirection)
    (if (< (Variables|Default|GetMovement%20speed/Direction) 0.0)
      (Variables|Default|SetMovement%20speed/Direction (* (Variables|Default|GetMovement%20speed/Direction) -1.0)))
    (elif (> (Variables|Default|GetMovement%20speed/Direction) 0.0)
      (Variables|Default|SetMovement%20speed/Direction (* (Variables|Default|GetMovement%20speed/Direction) -1.0))))
  (bind _output_get (Variables|Default|SetRandomMove (+ (Variables|Default|GetRandomMove) 1)))
  (if (> _output_get 200)
    (Variables|Default|SetMovement%20speed/Direction (* (Math|Random|RandomFloat) (Math|Random|RandomFloatinRange 2.0 6.0)))
    (Variables|Default|SetRandomMove 0)
    (Variables|Default|SetDirection (Math|Random|RandomBool))
    (else
      (if (Variables|Default|GetOverlappingSoft)
        (bind _as2dside_scroller_character (Utilities|Casting|CastTo2DSideScrollerCharacter (Game|Player|GetPlayerPawn 0))
          (:then
            (Default|GrowSoft _as2dside_scroller_character))
          (:CastFailed
            _)))
      (Transformation|AddActorWorldOffset (Math|Vector|MakeVector (Variables|Default|GetMovement%20speed/Direction) 0.0 0.0)))))

(fn ConstructionScript)